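; BP_Enemy_Animal is an animal enemy that wanders the level and chases pawns it sees.
; On BeginPlay it starts Roam, which moves to random navigable points via AIMoveTo, pausing and repeating after each success.
; PawnSensing sightings raise walk speed and start a chase; a retriggerable delay restores speed and resumes roaming after sightings stop.
; A similar Walk loop is defined but never called in this file.
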(event `self.ReceiveBeginPlay`
  (`self.Roam`))

(event `Roam`
  (bind _randomlocation (`NavigationSystemV1.K2_GetRandomLocationInNavigableRadius` (`self.K2_GetActorLocation`) 1000.0 null null))
  (`|AIMoveTo` self _randomlocation null
    (:`OnSuccess`
      (`KismetSystemLibrary.Delay` 4.0)
      (`self.Roam`))))

(event `Walk`
  (`|AIMoveTo` self (`NavigationSystemV1.K2_GetRandomReachablePointInRadius` (`self.K2_GetActorLocation`) 0.0 null null) null
    (:`OnSuccess`
      (`KismetSystemLibrary.Delay` 0.5)
      (`self.Walk`))))

(event `self.PawnSensing.OnSeePawn`
  (params (Pawn :type "Pawn Object Reference"))
  (`KismetSystemLibrary.PrintString` "Im coming")
  (set `CharacterMovementComponent.MaxWalkSpeed` 450.0 (`self.CharacterMovement`))
  (`|AIMoveTo` self (0.0 0.0 0.0) Pawn
    (:`then`
      (`KismetSystemLibrary.RetriggerableDelay` 5.0)
      (set `CharacterMovementComponent.MaxWalkSpeed` 250.0 (`self.CharacterMovement`))
      (`self.Roam`))))

(fn `UserConstructionScript`)