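; BP_Dizzy is a level actor that toggles a post-process effect, by its name a dizziness look, based on the player character's happiness.
; On BeginPlay it finds and caches the BP_ThirdPersonCharacter in the level.
; Each Tick it polls that character's HappyPoint, showing the PostProcess component only within a low band and hiding it above or below that band.
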(event `self.ReceiveTick`
  (params (DeltaSeconds :type "Float (single-precision)"))
  (bind _postprocess (`self.PostProcess`))
  (if (< (`/Game/ThirdPerson/Blueprints/BP_ThirdPersonCharacter.HappyPoint` (`self.Chara`)) 25.0)
    (`SceneComponent.SetVisibility` _postprocess true false)
    (if (< (`/Game/ThirdPerson/Blueprints/BP_ThirdPersonCharacter.HappyPoint` (`self.Chara`)) 10.0)
      (`SceneComponent.SetVisibility` _postprocess false false))
    (else
      (`SceneComponent.SetVisibility` _postprocess false false))))

(event `self.ReceiveBeginPlay`
  (bind _returnvalue (`GameplayStatics.GetActorOfClass` "/Game/ThirdPerson/Blueprints/BP_ThirdPersonCharacter.BP_ThirdPersonCharacter_C"))
  (set `self.Chara` _returnvalue))

(fn `UserConstructionScript`)