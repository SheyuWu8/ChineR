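; Fishing lure actor that attracts a fish and hooks it on contact.
; From BeginPlay it gathers fish overlapping CollideFish, retrying every two seconds until one is selected and told to approach via message.
; Selection measures actor-to-SphereAttract distance rather than distance to each fish.
; A fish entering SphereAttract is frozen, attached to the player's FishPole socket and reported to BP_ThirdPersonCharacter as caught.
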(event `self.ReceiveBeginPlay`
  (`self.FindNearestFish`))

(event `FindNearestFish`
  (bind _returnvalue (`KismetMathLibrary.Vector_Distance` (`self.K2_GetActorLocation`) (`SceneComponent.K2_GetComponentLocation` (`self.SphereAttract`))))
  (`/Engine/EditorBlueprintResources/StandardMacros.IsValid` (`self.NearestFish`)
    (:`Is Not Valid`
      (`KismetArrayLibrary.Array_Clear` (`self.FishAttracts`))
      (for _array_element (`PrimitiveComponent.GetOverlappingActors` (`self.CollideFish`) null)
        (bind _fish (message `/Game/Level/Fishing/BPI_Fish.isFish` _array_element))
        (if _fish
          (`KismetArrayLibrary.Array_Add` (`self.FishAttracts`) _array_element)))
      (for _array_element_2 (`self.FishAttracts`)
        (if (< _returnvalue (`self.NearestDistance`))
          (set `self.NearestDistance` _returnvalue)
          (set `self.NearestFish` _array_element_2)))
      (`self.AttractNearest` true)
      (`KismetSystemLibrary.Delay` 2.0)
      (`self.FindNearestFish`))))

(event `AttractNearest`
  (params (Attract :type Boolean))
  (bind _nearestfish (`self.NearestFish`))
  (`/Engine/EditorBlueprintResources/StandardMacros.IsValid` _nearestfish
    (:`Is Valid`
      (message `/Game/Level/Fishing/BPI_Fish.AttractFishing` _nearestfish Attract self))))

(event `self.SphereAttract.OnComponentBeginOverlap`
  (params (OverlappedComponent :type "PrimitiveComponent Object Reference") (OtherActor :type "Actor Object Reference") (OtherComp :type "PrimitiveComponent Object Reference") (OtherBodyIndex :type Integer) (bFromSweep :type Boolean) (SweepResult :type "HitResult Structure (by ref)"))
  (bind _fish (message `/Game/Level/Fishing/BPI_Fish.isFish` OtherActor))
  (if _fish
    (bind _output_get (set `self.CaughtFish` OtherActor))
    (`self.SetActorTickEnabled` _output_get false)
    (`PrimitiveComponent.SetCollisionEnabled` (`self.SphereAttract`) "NoCollision")
    (bind _asch_fish_1 (cast `/Game/Level/Fishing/CH_Fish1` _output_get))
    (`MovementComponent.StopMovementImmediately` (`Character.CharacterMovement` _asch_fish_1))
    (`SkeletalMeshComponent.SetAnimInstanceClass` (`Character.Mesh` _asch_fish_1) null)
    (bind _asbp_third_person_character (cast `/Game/ThirdPerson/Blueprints/BP_ThirdPersonCharacter` (`GameplayStatics.GetPlayerPawn` 0)))
    (`self.K2_AttachToComponent` (`self.CaughtFish`) (`/Game/ThirdPerson/Blueprints/BP_ThirdPersonCharacter.FishPole` _asbp_third_person_character) "attractorSocket" "SnapToTarget" "SnapToTarget" "KeepWorld" false)
    (`/Game/ThirdPerson/Blueprints/BP_ThirdPersonCharacter.CaughtFish` _asbp_third_person_character)))

(fn `UserConstructionScript`)