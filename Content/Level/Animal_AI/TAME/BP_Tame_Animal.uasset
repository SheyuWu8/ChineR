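; Tameable animal AI that wanders the navmesh, reacts to seen pawns and can follow the player once tamed.
; Self-repeating AIMoveTo events drive wander, flee and follow, each setting walk speed; completing a wander move clears the tamed state.
; Sighting while untamed triggers RunAway, offset along the look-at line to the player, then wandering after a retriggerable delay.
; Taming is a coin flip; failure blocks it until a later attempt starts a cooldown.
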(event `self.ReceiveBeginPlay`
  (`self.WalkAround`)
  (bind _asbp_third_person_character (cast `/Game/ThirdPerson/Blueprints/BP_ThirdPersonCharacter` (`GameplayStatics.GetPlayerCharacter` 0)))
  (set `self.Player` _asbp_third_person_character))

(event `WalkAround`
  ;[1 1 1] Walk Around
  (set `CharacterMovementComponent.MaxWalkSpeed` (`self.OriginSpeed`) (`self.CharacterMovement`))
  (`|AIMoveTo` self (`NavigationSystemV1.K2_GetRandomReachablePointInRadius` (`self.K2_GetActorLocation`) 500.0 null null) null
    (:`OnSuccess`
      (`KismetSystemLibrary.Delay` 3.0)
      (`self.WalkAround`)
      (set `self.FollowPlayer?` false)
      (set `self.Tame?` false))))

(event `Taming`
  (if (not (`self.Tame?`))
    (`MovementComponent.StopMovementImmediately` (`self.CharacterMovement`))
    (`self.FollowPlayer`)
    (set `self.Tame?` true)
    (set `self.FollowPlayer?` true)))

(event `/Game/Level/Animal_AI/BPI_Animal.Tame`
  (if (`self.CanTame`)
    (if (`KismetMathLibrary.RandomBool`)
      (`KismetSystemLibrary.PrintString` "YesSir")
      (`self.Taming`)
      (else
        (`KismetSystemLibrary.PrintString` "NoCanDO")
        (set `self.CanTame` false)))
    (else
      (`KismetSystemLibrary.PrintString` "not now")
      (`KismetSystemLibrary.Delay` 3.0)
      (set `self.CanTame` true))))

(event `FollowPlayer`
  ;[1 1 1] FollowPlayer
  (set `CharacterMovementComponent.MaxWalkSpeed` (`self.FollowingSpeed`) (`self.CharacterMovement`))
  (`|AIMoveTo` self (0.0 0.0 0.0) (`GameplayStatics.GetPlayerCharacter` 0) 200.0
    (:`OnSuccess`
      (`KismetSystemLibrary.Delay` 0.5)
      (if (`self.FollowPlayer?`)
        (`self.FollowPlayer`)))))

(event `ToggleStateAI`)

(event `RunAway`
  (bind _returnvalue (`self.K2_GetActorLocation`))
  (bind (_x _y) (`KismetMathLibrary.BreakVector3f` (+ _returnvalue (* (`KismetMathLibrary.GetForwardVector` (`KismetMathLibrary.FindLookAtRotation` _returnvalue (`self.K2_GetActorLocation` (`self.Player`)))) (`self.RunAwayDistance`)))))
  (set `CharacterMovementComponent.MaxWalkSpeed` (`self.MaxSpeed`) (`self.CharacterMovement`))
  (`|AIMoveTo` self (`NavigationSystemV1.K2_GetRandomReachablePointInRadius` (`KismetMathLibrary.MakeVector` _x _y (`.Z` (`KismetMathLibrary.BreakVector3f` _returnvalue))) 1000.0 null null) null
    (:`OnSuccess`
      (`self.RunAway`))))

(event `self.PawnSensing.OnSeePawn`
  (params (Pawn :type "Pawn Object Reference"))
  (if (`self.Tame?`)
    (`KismetSystemLibrary.PrintString` "following")
    (else
      (`KismetSystemLibrary.PrintString` "ahhhhhhhhhhhhhhhhhhh")
      (`self.RunAway`)
      (`KismetSystemLibrary.RetriggerableDelay` 2.0)
      (`self.WalkAround`))))

(fn `UserConstructionScript`)