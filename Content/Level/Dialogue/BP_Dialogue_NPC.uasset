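; Dialogue NPC that talks to the player line by line and grants the flashlight at the third line.
; A sphere overlap toggles a widget component when the player character approaches or leaves.
; Each Talk call advances the index, updates a reused WBP_Dialogue and plays the matching sound, hiding and restarting after the last line.
; The Talkkkkk function and random-voice logic are disconnected leftovers.
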(event `/Game/Level/Dialogue/BPI_Dialogue.Talk`
  (bind _ui (`self.UI`))
  ;[1 1 1] Set Text UI
  (`/Engine/EditorBlueprintResources/StandardMacros.IncrementInt` (`self.TalkIndex`)
    (:`  `
      (if (< (`self.TalkIndex`) (`KismetArrayLibrary.Array_Length` (`self.Dialogue`)))
        (`self.UI`
          (:`then`
            (`Widget.SetVisibility` _ui "Visible"))
          (:`else`
            (bind _returnvalue (`|CreateWidget` "/Game/UI/UI_Dialogue/WBP_Dialogue.WBP_Dialogue_C" (`GameplayStatics.GetPlayerController` 0)))
            (bind _output_get (set `self.UI` _returnvalue))
            (`UserWidget.AddToViewport` _output_get 0)))
        (`TextBlock.SetText` (`/Game/UI/UI_Dialogue/WBP_Dialogue.TalkText` _ui) (`KismetTextLibrary.Conv_StringToText` (`|GetArrayItem` (`self.Dialogue`) (`self.TalkIndex`))))
        (`GameplayStatics.PlaySound2D` (`|GetArrayItem` (`self.SoundBase`) (`self.TalkIndex`)) 1.0 1.0 0.0 null null)
        (if (== (`self.TalkIndex`) 2)
          (bind _asbp_third_person_character (cast `/Game/ThirdPerson/Blueprints/BP_ThirdPersonCharacter` (`GameplayStatics.GetPlayerCharacter` 0)))
          (set `/Game/ThirdPerson/Blueprints/BP_ThirdPersonCharacter.flashLightGiven` true _asbp_third_person_character))
        (else
          (`Widget.SetVisibility` (`self.UI`) "Hidden")
          (set `self.TalkIndex` -1))))))

(event `self.Sphere.OnComponentBeginOverlap`
  (params (OverlappedComponent :type "PrimitiveComponent Object Reference") (OtherActor :type "Actor Object Reference") (OtherComp :type "PrimitiveComponent Object Reference") (OtherBodyIndex :type Integer) (bFromSweep :type Boolean) (SweepResult :type "HitResult Structure (by ref)"))
  (cast `/Game/ThirdPerson/Blueprints/BP_ThirdPersonCharacter` OtherActor)
  (`SceneComponent.SetVisibility` (`self.Widget`) true false))

(event `self.Sphere.OnComponentEndOverlap`
  (params (OverlappedComponent :type "PrimitiveComponent Object Reference") (OtherActor :type "Actor Object Reference") (OtherComp :type "PrimitiveComponent Object Reference") (OtherBodyIndex :type Integer))
  (`SceneComponent.SetVisibility` (`self.Widget`) false false))

(fn `talkkkkk`
  (`/Engine/EditorBlueprintResources/StandardMacros.IncrementInt` (`self.TalkIndex`)
    (:`  `
      (if (< (`self.TalkIndex`) (`KismetArrayLibrary.Array_Length` (`self.Dialogue`)))
        (`self.UI`
          (:`then`
            _)
          (:`else`
            (bind _returnvalue (`|CreateWidget` "/Game/UI/UI_Dialogue/WBP_Dialogue.WBP_Dialogue_C" (`GameplayStatics.GetPlayerController` 0)))
            (bind _output_get (set `self.UI` _returnvalue))
            (`UserWidget.AddToViewport` _output_get 0)))
        (`TextBlock.SetText` (`/Game/UI/UI_Dialogue/WBP_Dialogue.TalkText` (`self.UI`)) (`KismetTextLibrary.Conv_StringToText` (`|GetArrayItem` (`self.Dialogue`) (`self.TalkIndex`))))
        (if (< (`self.TalkIndex`) (`KismetArrayLibrary.Array_Length` (`self.Dialogue`)))
          (if (== (`self.TalkIndex`) 0)
            (`AudioComponent.Play` (`self.你好`) 0.0)
            (elif (== (`self.TalkIndex`) 1)
              (`AudioComponent.Play` (`self.盖亚`) 0.0)
              (set `self.FinishTalk` true))))
        (else
          (`Widget.RemoveFromParent` (`self.UI`)))))))

(fn `UserConstructionScript`)