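; BP_SpawnPlant is a level spawner that lays out a grid of BP_PickUp actors on the surface beneath it at BeginPlay.
; SPAWN runs nested X/Y loops from the actor's location, firing debug-drawn Visibility traces along its down vector at evenly spaced points.
; Each hit spawns a pickup slightly above the impact, with an extra row from the outer loop's own trace.
; A disconnected BP_Roster spawn loop never runs.
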(event `self.ReceiveBeginPlay`
  (`self.SPAWN`))

(event `SPAWN`
  (bind (_returnvalue_x _returnvalue_y _returnvalue_z) (`KismetMathLibrary.BreakVector` (`self.K2_GetActorLocation`)))
  (bind (_returnvalue_x_2 _returnvalue_y_2 _returnvalue_z_2) (`KismetMathLibrary.BreakVector` (`self.K2_GetActorLocation`)))
  ;[1 1 1] X
  (for _index (range 1 11)
    (bind _returnvalue (+ (* _index 50) _returnvalue_x))
    (bind _returnvalue_2 (`KismetMathLibrary.MakeVector` _returnvalue _returnvalue_y _returnvalue_z))
    (bind (_outhit _returnvalue_3) (`KismetSystemLibrary.LineTraceSingle` :`Start` _returnvalue_2 :`End` (+ _returnvalue_2 (* (`KismetMathLibrary.GetUpVector` (`self.K2_GetActorRotation`)) -5000.0)) :`TraceChannel` "TraceTypeQuery1" :`DrawDebugType` "ForDuration"))
    (`|ExecutionSequence`
      (:`then_0`
        ;[1 1 1] Y
        (for _index_2 (range 1 11)
          (bind _returnvalue_4 (`KismetMathLibrary.MakeVector` _returnvalue (+ (* _index_2 50) _returnvalue_y_2) _returnvalue_z_2))
          (bind (_outhit_2 _returnvalue_5) (`KismetSystemLibrary.LineTraceSingle` :`Start` _returnvalue_4 :`End` (+ _returnvalue_4 (* (`KismetMathLibrary.GetUpVector` (`self.K2_GetActorRotation`)) -5000.0)) :`TraceChannel` "TraceTypeQuery1" :`DrawDebugType` "ForDuration"))
          (if _returnvalue_5
            (`|SpawnActorFromClass` "/Game/Level/Inventory/BP_PickUp.BP_PickUp_C" (`KismetMathLibrary.MakeTransform` (+ (`.Location` (`GameplayStatics.BreakHitResult` _outhit_2)) (0.0 0.0 100.0))) "AlwaysSpawn" "MultiplyWithRoot" null null))))
      (:`then_1`
        (if _returnvalue_3
          (`|SpawnActorFromClass` "/Game/Level/Inventory/BP_PickUp.BP_PickUp_C" (`KismetMathLibrary.MakeTransform` (+ (`.Location` (`GameplayStatics.BreakHitResult` _outhit)) (0.0 0.0 100.0))) "AlwaysSpawn" "MultiplyWithRoot" null null))))))

(fn `UserConstructionScript`)