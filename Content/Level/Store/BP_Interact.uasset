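; BP_Interact is an interactable store point that shows a prompt near the player and can open the store UI.
; Its Sphere shows the Widget component when a BP_ThirdPersonCharacter begins overlapping and hides it when any overlap ends, without checking the actor.
; The OpenStore event, not called within this graph, adds a new WBP_Store to the viewport, shows the cursor and focuses it in Game and UI input mode.
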(event `self.Sphere.OnComponentBeginOverlap`
  (params (OverlappedComponent :type "PrimitiveComponent Object Reference") (OtherActor :type "Actor Object Reference") (OtherComp :type "PrimitiveComponent Object Reference") (OtherBodyIndex :type Integer) (bFromSweep :type Boolean) (SweepResult :type "HitResult Structure (by ref)"))
  (cast `/Game/ThirdPerson/Blueprints/BP_ThirdPersonCharacter` OtherActor)
  (`SceneComponent.SetVisibility` (`self.Widget`) true false))

(event `self.Sphere.OnComponentEndOverlap`
  (params (OverlappedComponent :type "PrimitiveComponent Object Reference") (OtherActor :type "Actor Object Reference") (OtherComp :type "PrimitiveComponent Object Reference") (OtherBodyIndex :type Integer))
  (`SceneComponent.SetVisibility` (`self.Widget`) false false))

(event `OpenStore`
  (bind _returnvalue (`GameplayStatics.GetPlayerController` 0))
  (bind _returnvalue_2 (`|CreateWidget` "/Game/UI/UI_interact_Store/WBP_Store.WBP_Store_C"))
  (bind _output_get (set `self.StoreWidget` _returnvalue_2))
  (`UserWidget.AddToViewport` _output_get 0)
  (set `PlayerController.bShowMouseCursor` true _returnvalue)
  (`WidgetBlueprintLibrary.SetInputMode_GameAndUIEx` _returnvalue (`self.StoreWidget`)))

(fn `UserConstructionScript`)